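; Game state Blueprint for SideRooms that places players at game start and serves as a test spot for things like map generation.
; Its InitGame event runs the parent logic, then adds player characters 0 and 1 to CharacterArray.
; Each valid character is teleported to a randomly indexed entry in SpawnLocationArray, with no check against shared spots.
; The random range's upper bound is the array length, so the index can fall out of bounds.
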(event `self.InitGame`
  (bind _characterarray (`self.CharacterArray`))
  (bind _spawnlocationarray (`self.SpawnLocationArray`))
  ;[1 1 1] 맵 생성 같은거 여기서 테스트 하세요
  (`parent.InitGame`)
  (`KismetArrayLibrary.Array_Add` _characterarray (`GameplayStatics.GetPlayerCharacter` 0))
  (`KismetArrayLibrary.Array_Add` _characterarray (`GameplayStatics.GetPlayerCharacter` 1))
  ;[1 1 1] InitPlayer()
  (for _array_element _characterarray
    (`/Engine/EditorBlueprintResources/StandardMacros.IsValid` _array_element
      (:`Is Valid`
        (`self.K2_SetActorLocation` _array_element (`|GetArrayItem` _spawnlocationarray (`KismetMathLibrary.RandomIntegerInRange` 0 (`KismetArrayLibrary.Array_Length` _spawnlocationarray))) false true)))))

(fn `UserConstructionScript`)