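; BP_Component_Rifle is a rifle weapon component whose Blueprint graph only adds an on-screen debug readout of weapon state.
; Each Tick prints clip size with current ammo, plus the can-fire and reloading flags, in two colors.
; Print durations follow DeltaSeconds so the text refreshes every frame, and log output is off.
; BeginPlay is empty, and no firing or reload logic appears in this graph.
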(event `self.ReceiveTick`
  (params (DeltaSeconds :type "Float (single-precision)"))
  (bind _returnvalue (+ DeltaSeconds 0.002))
  (`KismetSystemLibrary.PrintString` (`KismetStringLibrary.Concat_StrStr` "Ammo : " (`KismetStringLibrary.Conv_IntToString` (`self.GetCurrentClipSize`)) " / " (`KismetStringLibrary.Conv_IntToString` (`self.GetCurrentAmmo`))) true false (struct :`R` 1.0 :`G` 0.280043 :`B` 0.319854 :`A` 1.0) _returnvalue)
  (`KismetSystemLibrary.PrintString` (`KismetStringLibrary.Concat_StrStr` "bCanFire : " (`KismetStringLibrary.Conv_BoolToString` (`self.GetCanFire`)) " / " "bIsReloading : " (`KismetStringLibrary.Conv_BoolToString` (`self.GetIsReloading`))) true false (struct :`R` 1.0 :`G` 0.818089 :`B` 0.159794 :`A` 1.0) _returnvalue))