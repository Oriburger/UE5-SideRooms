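; BP_SideRoomPlayerController is a player controller that lets the host start a SideRooms match with the Enter key.
; On Enter with authority, it calls StartGame on SideRoomsGameMode and a server event that spawns a rifle pickup at a fixed spot near the world origin.
; The pickup's owner is then set to player controller 0.
; InitHUD_1 is empty, and the WB_MainHUD creation logic is disconnected.
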(event `InitHUD_1`
  ;[1 1 1] HUD
)

(event `Key|Enter` :consume false
  (params (Key :type "Key Structure"))
  (:`Pressed`
    (if (`self.HasAuthority`)
      (bind _asside_rooms_game_mode (cast `SideRoomsGameMode` (`GameplayStatics.GetGameMode`)))
      (`SideRoomsGameMode.StartGame` _asside_rooms_game_mode)
      (`self.ServerRPCSpawnItem`))))

(event `ServerRPCSpawnItem`
  (`self.SpawnItem`))

(event `SpawnItem`
  (bind _returnvalue (`|SpawnActorFromClass` "/Game/Weapon/Blueprint/BP_PickUp_Rifle.BP_PickUp_Rifle_C" (`KismetMathLibrary.MakeTransform` (0.0 0.0 60.0)) "Undefined" "MultiplyWithRoot" self null))
  (`self.SetOwner` _returnvalue (`GameplayStatics.GetPlayerController` 0)))

(fn `UserConstructionScript`)