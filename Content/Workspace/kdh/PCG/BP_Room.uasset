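; BP_Room is a room actor in the PCG folder that randomizes which of its walls are present.
; Its Construction Script rolls a random float for each of four wall components and destroys any at or above WallPercentage, making that value the chance a wall stays.
; A disconnected branch for random decal material or removal never runs, and the Event Graph holds only empty default events.
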(event EventBeginPlay)

(event Collision|EventActorBeginOverlap
  (params (OtherActor :type Actor%20Object%20Reference)))

(event EventTick
  (params (DeltaSeconds :type Float%20%28single-precision%29)))

(fn ConstructionScript
  (for _array_element (Utilities|Array|MakeArray (Variables|Default|GetWall) (Variables|Default|GetWall1) (Variables|Default|GetWall2) (Variables|Default|GetWall3))
    (if (>= (Math|Random|RandomFloat) (Variables|Default|GetWallPercentage))
      (Components|DestroyComponent _array_element))))