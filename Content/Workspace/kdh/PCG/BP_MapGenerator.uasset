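; BP_MapGenerator is an actor that builds a grid-based room map at BeginPlay, spaced by RoomInterval from its own location.
; Nested loops over Width and Height, padded for a border, spawn BP_Wall on the edges, BP_Room inside and BP_SpawnRoom at the half-Width, half-Height cell.
; Spawned rooms and walls attach to the generator.
; A PlayerStart spawned above the spawn room is used to restart player 0 there.
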(event EventBeginPlay
  (bind _returnvalue (Transformation|GetActorLocation))
  (bind _roominterval (Variables|Default|GetRoomInterval))
  (bind _defaultsceneroot (Variables|Default|GetDefaultSceneRoot))
  (bind _returnvalue_2 (Components|GetOwner _defaultsceneroot))
  (for _index (range 0 (+ (Variables|Default|GetWidth) 2))
    (for _index_2 (range 0 (+ (Variables|Default|GetHeight) 2))
      ;[1 1 1] Spawn 위치
      (if (and (== (/ (Variables|Default|GetWidth) 2) _index) (== (/ (Variables|Default|GetHeight) 2) _index_2))
        (bind _returnvalue_3 (Game|SpawnActorfromClass "/Game/Workspace/kdh/PCG/BP_SpawnRoom.BP_SpawnRoom_C" (Math|Conversions|ToTransform(Vector) (Math|Vector|MakeVector (+ (Math|Conversions|ToFloat(Integer) (* _index _roominterval)) (.x _returnvalue)) (+ (Math|Conversions|ToFloat(Integer) (* _index_2 _roominterval)) (.y _returnvalue)) (.z _returnvalue))) "Undefined" "MultiplyWithRoot" 0 0))
        (Transformation|AttachActorToActor _returnvalue_3 _returnvalue_2 "Rooms" "KeepRelative" "KeepRelative" "KeepRelative" true)
        (bind _returnvalue_4 (Game|SpawnActorfromClass "/Script/Engine.PlayerStart" (Math|Conversions|ToTransform(Vector) (Math|Vector|MakeVector (+ (Math|Conversions|ToFloat(Integer) (* _index _roominterval)) (.x _returnvalue)) (+ (Math|Conversions|ToFloat(Integer) (* _index_2 _roominterval)) (.y _returnvalue)) (+ (.z _returnvalue) 8e+01))) "Undefined" "MultiplyWithRoot" 0 0))
        (Class|GameModeBase|RestartPlayeratPlayerStart (Game|GetGameMode) (Game|GetPlayerController 0) _returnvalue_4)
        (elif (or (or (== _index 0) (== _index_2 0)) (or (== _index (+ (Variables|Default|GetWidth) 2)) (== _index_2 (+ (Variables|Default|GetHeight) 2))))
          (bind _returnvalue_5 (Game|SpawnActorfromClass "/Game/Workspace/kdh/PCG/BP_Wall.BP_Wall_C" (Math|Conversions|ToTransform(Vector) (Math|Vector|MakeVector (+ (Math|Conversions|ToFloat(Integer) (* _index _roominterval)) (.x _returnvalue)) (+ (Math|Conversions|ToFloat(Integer) (* _index_2 _roominterval)) (.y _returnvalue)) (.z _returnvalue))) "Undefined" "MultiplyWithRoot" 0 0))
          (Transformation|AttachActorToActor _returnvalue_5 _returnvalue_2 "Rooms" "KeepRelative" "KeepRelative" "KeepRelative" true)
          (else
            (bind _returnvalue_6 (Game|SpawnActorfromClass "/Game/Workspace/kdh/PCG/BP_Room.BP_Room_C" (Math|Conversions|ToTransform(Vector) (Math|Vector|MakeVector (+ (Math|Conversions|ToFloat(Integer) (* _index _roominterval)) (.x _returnvalue)) (+ (Math|Conversions|ToFloat(Integer) (* _index_2 _roominterval)) (.y _returnvalue)) (.z _returnvalue))) "Undefined" "MultiplyWithRoot" 0 0))
            (Transformation|AttachActorToActor _returnvalue_6 _returnvalue_2 "Rooms" "KeepRelative" "KeepRelative" "KeepRelative" true)))))))

(event Collision|EventActorBeginOverlap
  (params (OtherActor :type Actor%20Object%20Reference)))

(event EventTick
  (params (DeltaSeconds :type Float%20%28single-precision%29)))

(fn ConstructionScript)