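; BP_Target is a target prop that pitches over when it takes any damage, then resets itself.
; AnyDamage calls the RotateAnimationOnClient event, which plays a timeline from the start to drive the root component's relative pitch.
; When that finishes, a three-second delay leads into a second timeline played in reverse from its end, driving the same pitch.
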(event `self.ReceiveAnyDamage`
  (params (Damage :type "Float (single-precision)") (DamageType :type "DamageType Object Reference") (InstigatedBy :type "Controller Object Reference") (DamageCauser :type "Actor Object Reference"))
  (`self.RotateAnimationOnClient`))

(event `RotateAnimationOnClient`
  (bind (_direction `_새_트랙_0`) (`Timeline|타임라인` :!via `PlayFromStart`)
    (:`Update`
      (`SceneComponent.K2_SetRelativeRotation` (`self.DefaultSceneRoot`) (`KismetMathLibrary.MakeRotator` 0.0 `_새_트랙_0`) false false))
    (:`Finished`
      (`KismetSystemLibrary.Delay` 3.0)
      (bind (_direction_2 `_새_트랙_0_2`) (`Timeline|타임라인_0` :!via `ReverseFromEnd`)
        (:`Update`
          (`SceneComponent.K2_SetRelativeRotation` (`self.DefaultSceneRoot`) (`KismetMathLibrary.MakeRotator` 0.0 `_새_트랙_0_2`) false false))))))

(fn `UserConstructionScript`)